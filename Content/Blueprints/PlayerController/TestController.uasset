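; Test player controller that saves a Team value to a save game through the custom event SaveMyStuffPlease.
; If the "self" slot exists, it loads the SaveMyInfoBP, sets Team, saves it back and prints the success result.
; Otherwise it only creates a save object, as the chain that would set Team and save it is disconnected, so no first save is written.
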(event Custom|SaveMyStuffPlease
  (params (Team :type Boolean))
  (bind _returnvalue (SaveGame|DoesSaveGameExist "self"))
  (if _returnvalue
    (bind _returnvalue_2 (SaveGame|LoadGamefromSlot "self"))
    (bind _output_get (Variables|Default|SetSelfSave _returnvalue_2))
    (bind _assave_my_info_bp (Utilities|Casting|CastToSaveMyInfoBP _output_get))
    (Variables|/Game/Blueprints/TeamSetup/SaveMyInfoBP.SaveMyInfoBP_C|SetTeam _assave_my_info_bp Team)
    (bind _returnvalue_3 (SaveGame|SaveGametoSlot (Variables|Default|GetSelfSave) "Self"))
    (Development|PrintString (Utilities|String|ToString(Boolean) _returnvalue_3) true true "(R=0.525000,G=0.000000,B=0.020877,A=1.000000)")
    (else
      (bind _returnvalue_4 (SaveGame|CreateSaveGameObject "/Game/Blueprints/TeamSetup/SaveMyInfoBP.SaveMyInfoBP_C")))))

(event EventBeginPlay)

(event EventTick
  (params (DeltaSeconds :type Float%20%28single-precision%29)))

(fn ConstructionScript)
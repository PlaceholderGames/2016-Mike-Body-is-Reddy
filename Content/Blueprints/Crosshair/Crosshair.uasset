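; Crosshair is a HUD Blueprint that draws a small dark green square as a crosshair near the screen center.
; DrawHUD halves the canvas size and uses that point as the square's top-left corner, with no offset for its own size.
; An unconnected custom crosshair branch would draw a material around the DPI-scaled mouse position, but it never runs.
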(event EventBeginPlay)

(event Collision|EventActorBeginOverlap
  (params (OtherActor :type Actor%20Object%20Reference)))

(event EventDrawHUD
  (params (SizeX :type Integer) (SizeY :type Integer))
  (HUD|DrawRect self "(R=0.053272,G=0.200000,B=0.037754,A=1.000000)" (Math|Conversions|ToFloat(Integer) (/ SizeX 2)) (Math|Conversions|ToFloat(Integer) (/ SizeY 2)) 5.0 5.0))

(event EventTick
  (params (DeltaSeconds :type Float%20%28single-precision%29)))

(fn ConstructionScript)
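; A one-meter cube actor, by its name, that prints "Hello" to the screen while a Character overlaps it.
; Begin and end overlap events set and clear an Overlapping flag for Characters, and Tick prints every frame while it is set.
; The flag is a single boolean, so any Character leaving clears it, and its RepNotify function is empty.
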(event EventBeginPlay
  (Variables|Default|Setoverlapping false))

(event Collision|EventActorBeginOverlap
  (params (OtherActor :type Actor%20Object%20Reference))
  (Utilities|Casting|CastToCharacter OtherActor)
  (Variables|Default|Setoverlapping true))

(event EventTick
  (params (DeltaSeconds :type Float%20%28single-precision%29))
  (if (Variables|Default|Getoverlapping)
    (Development|PrintString "Hello")))

(event Collision|EventActorEndOverlap
  (params (OtherActor :type Actor%20Object%20Reference))
  (Utilities|Casting|CastToCharacter OtherActor)
  (Variables|Default|Setoverlapping false))

(fn ConstructionScript)

(fn OnRepOverlapping)